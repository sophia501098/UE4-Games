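; M4A1 weapon Blueprint that implements hitscan firing through its Fire event.
; Fire line-traces on the Visibility channel from the mesh's GunExitSocket along the socket's forward vector, out to WeaponStatus.Range, with debug drawing on.
; A hit applies WeaponStatus.Damage as small-radius radial damage at the hit location, credited to the instigator's controller, and prints the instigator's name for debugging.
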(event Custom|Fire
  (bind _staticmesh (Variables|Default|GetStaticMesh))
  (bind _returnvalue (Transformation|GetSocketLocation _staticmesh "GunExitSocket"))
  (bind (_outhit _returnvalue_2) (Collision|LineTraceByChannel _returnvalue (+ _returnvalue (* (Math|Vector|GetForwardVector (Transformation|GetSocketRotation _staticmesh "GunExitSocket")) (.range (Variables|Default|GetWeapon%20Status)))) "TraceTypeQuery1" false 0 "ForDuration"))
  (if _returnvalue_2
    (Game|Damage|ApplyRadialDamage (.damage (Variables|Default|GetWeapon%20Status)) (.Location (Collision|BreakHitResult _outhit)) 1e+01 0 0 self (Game|GetInstigatorController) false "ECC_Visibility")
    (Development|PrintString (Utilities|GetDisplayName (Game|GetInstigator)))))

(event EventBeginPlay)

(event Collision|EventActorBeginOverlap
  (params (OtherActor :type Actor%20Object%20Reference)))

(event EventTick
  (params (DeltaSeconds :type Float%20%28single-precision%29)))

(fn ConstructionScript)